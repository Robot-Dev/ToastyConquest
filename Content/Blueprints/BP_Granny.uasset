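; BP_Granny is the Granny boss actor, whose removal from play marks the player's victory.
; On BeginPlay it shows a Granny widget linked to itself and caches the relative locations of its teeth and eye spawn points.
; EndPlay, without checking the reason, removes the widget, spawns BP_DeadGranny in its place, plays victory music and destroys all remaining EnemyProjectile actors.
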(event EventBeginPlay
  (bind _returnvalue (UserInterface|CreateWidget "/Game/HUD/Granny.Granny_C" (Game|GetPlayerController 0)))
  (Variables|/Game/HUD/Granny.Granny_C|SetGranny _returnvalue self)
  (UserInterface|Viewport|AddtoViewport _returnvalue 0)
  (Variables|Default|SetTeethSpawnLocation (Variables|/Script/Engine.SceneComponent|GetRelativeLocation (Variables|Default|GetTeethSpawnLoc)))
  (Variables|Default|SetEyeSpawnLocation (Variables|/Script/Engine.SceneComponent|GetRelativeLocation (Variables|Default|GetEyeSpawnLoc))))

(event EventEndPlay
  (params (EndPlayReason :type EEndPlayReason%20Enum :default "Destroyed"))
  (Widget|RemovefromParent (stale EventBeginPlay _returnvalue))
  (Game|SpawnActorfromClass "/Game/Blueprints/BP_DeadGranny.BP_DeadGranny_C" (Transformation|GetActorTransform) "AlwaysSpawn" 0 0)
  (Audio|PlaySound2D "/Game/Sounds/Music/music_victory_v1_Cue.music_victory_v1_Cue")
  (bind _outactors (Actor|GetAllActorsOfClass "/Script/ToastyConquest.EnemyProjectile"))
  (for _array_element _outactors
    (Actor|DestroyActor _array_element)))

(fn ConstructionScript)