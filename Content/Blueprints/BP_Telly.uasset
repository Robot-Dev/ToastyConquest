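; BP_Telly is a hackable TV in a 2D toaster game that, when hacked, plays a cutscene waking a snoring Granny.
; OnHacked halts the Toaster, disables input and swaps the TV's flipbook and sound to the hacked state.
; Timelines lerp the side-view camera to Granny and back, with her stand-up flipbook replaced by a spawned BP_Granny in between.
; Afterwards, input returns and the blocking volume moves.
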(event EventBeginPlay
  (Audio|Components|Audio|Stop (Variables|Default|GetTellyHacked)))

(event EventOnHacked
  (bind _returnvalue (Game|GetPlayerController 0))
  (bind _granny (Variables|Default|GetGranny))
  (bind _granny_2 (Variables|Default|GetGranny))
  (bind _timedelay (Variables|Default|GetTimeDelay))
  (bind _returnvalue_2 (Transformation|GetWorldLocation _granny))
  (bind (_x _y _z) (Math|Vector|BreakVector _returnvalue_2))
  (bind (_x_2 _y_2 _z_2) (Math|Vector|BreakVector _returnvalue_2))
  (bind _astoaster (Utilities|Casting|CastToToaster (Pawn|GetControlledPawn _returnvalue)))
  (bind _astoaster_controller (Utilities|Casting|CastToToasterController _returnvalue))
  (Components|Movement|StopMovementImmediately (Variables|/Script/Engine.Character|GetCharacterMovement _astoaster))
  (Input|DisableInput _astoaster_controller 0)
  (Utilities|FlowControl|Delay 1.0)
  (Sprite|SetFlipbook (Variables|Default|GetSprite) "/Game/Sprites/Rooms/LivingRoom/Sprites/Telly_Hacked.Telly_Hacked")
  (Sprite|SetFlipbook (Variables|Default|GetHackable) "/Game/Sprites/Enemies/Granny/Death/Empty.Empty")
  (Audio|Components|Audio|Stop (Variables|Default|GetTellyIdle))
  (Audio|Components|Audio|Play (Variables|Default|GetTellyHacked) 0.0)
  (Utilities|FlowControl|Delay 1.0)
  (Variables|Default|SetStartWorldLocation (Transformation|GetWorldLocation (Variables|/Script/ToastyConquest.Toaster|GetSideViewCameraComponent _astoaster)))
  (bind _camera_movement (Timeline|Camera%20Movement%20Timeline Play)
    (:Update
      (Transformation|SetWorldLocation (Variables|/Script/ToastyConquest.Toaster|GetSideViewCameraComponent _astoaster) (Math|Vector|MakeVector (+ (* (- _x (.X (Math|Vector|BreakVector (Variables|Default|GetStartWorldLocation)))) _camera_movement) (.X (Math|Vector|BreakVector (Variables|Default|GetStartWorldLocation)))) (.Y (Math|Vector|BreakVector (Variables|Default|GetStartWorldLocation))) (+ (* (- _z (.Z (Math|Vector|BreakVector (Variables|Default|GetStartWorldLocation)))) _camera_movement) (.Z (Math|Vector|BreakVector (Variables|Default|GetStartWorldLocation))))) false false))
    (:Finished
      (Sprite|SetFlipbook _granny_2 "/Game/Sprites/Enemies/Granny/StandingUp/Granny_StandingUp.Granny_StandingUp")
      (Utilities|FlowControl|Delay _timedelay)
      (Sprite|SetFlipbook _granny_2 "/Game/Sprites/Enemies/Granny/Death/Empty.Empty")
      (Audio|Components|Audio|FadeOut (Variables|Default|GetGrannySnore) 0.5 0.0 :!class /Script/Engine.AudioComponent)
      (Audio|Components|Audio|FadeOut (Variables|Default|GetTellyHacked) 1.0 0.0 :!class /Script/Engine.AudioComponent)
      (Game|SpawnActorfromClass "/Game/Blueprints/BP_Granny.BP_Granny_C" (Math|Transform|MakeTransform _returnvalue_2) "AlwaysSpawn" 0 0)
      (Utilities|FlowControl|Delay (- 1.0 _timedelay))
      (bind _camera_movement_2 (Timeline|Camera%20Return%20Timeline Play)
        (:Update
          (Transformation|SetWorldLocation (Variables|/Script/ToastyConquest.Toaster|GetSideViewCameraComponent _astoaster) (Math|Vector|MakeVector (+ (* (- _x_2 (.X (Math|Vector|BreakVector (Variables|Default|GetStartWorldLocation)))) _camera_movement_2) (.X (Math|Vector|BreakVector (Variables|Default|GetStartWorldLocation)))) (.Y (Math|Vector|BreakVector (Variables|Default|GetStartWorldLocation))) (+ (* (- _z_2 (.Z (Math|Vector|BreakVector (Variables|Default|GetStartWorldLocation)))) _camera_movement_2) (.Z (Math|Vector|BreakVector (Variables|Default|GetStartWorldLocation))))) false false))
        (:Finished
          (Input|EnableInput _astoaster_controller 0)
          (Transformation|SetRelativeLocation (Variables|Default|GetBlockingVolume) "-500.000000, 0, 0" false false))))))

(fn ConstructionScript)