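; BP_Life is a health pickup that activates when a Toaster below max health overlaps its sphere.
; It deactivates, stores its start position and plays a timeline whose MoveTo value scales the offset from the Toaster's live position, so the motion tracks the moving target.
; When the timeline finishes, it adds one health to the Toaster, plays a life sound and destroys itself.
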(event OnComponentBeginOverlap(Sphere)
  (params (OverlappedComponent :type Primitive%20Component%20Object%20Reference) (OtherActor :type Actor%20Object%20Reference) (OtherComp :type Primitive%20Component%20Object%20Reference) (OtherBodyIndex :type Integer) (bFromSweep :type Boolean) (SweepResult :type Hit%20Result%20Structure%20%28by%20ref%29))
  (if (Variables|Default|GetbActive)
    (bind _astoaster (Utilities|Casting|CastToToaster OtherActor))
    (if (< (Variables|/Script/ToastyConquest.Toaster|GetHealth _astoaster) (Variables|/Script/ToastyConquest.Toaster|GetMaxHealth _astoaster))
      (Variables|Default|SetbActive false)
      (bind _output_get (Variables|Default|SetStartLocation (Transformation|GetActorLocation)))
      (bind _moveto (Timeline|Timeline_0 Play)
        (:Update
          (Transformation|SetActorLocation (+ (Transformation|GetActorLocation _astoaster) (* (- _output_get (Transformation|GetActorLocation _astoaster)) _moveto)) false false))
        (:Finished
          (Variables|/Script/ToastyConquest.Toaster|SetHealth _astoaster (+ (Variables|/Script/ToastyConquest.Toaster|GetHealth _astoaster) 1.0))
          (Audio|PlaySoundatLocation "/Game/Sounds/Other/asset_life_v1_Cue.asset_life_v1_Cue" (Transformation|GetActorLocation))
          (Actor|DestroyActor))))))

(fn ConstructionScript)