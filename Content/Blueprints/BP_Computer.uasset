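; BP_Computer is a hackable computer that ends the current level and sends the game to the Outro level.
; When hacked, it stops the player's Toaster pawn, disables input on the ToasterController and waits briefly.
; It then creates a LoadingScreen widget, pauses the game and opens Outro, with no step that adds the widget to the viewport.
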(event EventOnHacked
  (bind _returnvalue (Game|GetPlayerController 0))
  (bind _astoaster (Utilities|Casting|CastToToaster (Pawn|GetControlledPawn _returnvalue)))
  (bind _astoaster_controller (Utilities|Casting|CastToToasterController _returnvalue))
  (Components|Movement|StopMovementImmediately (Variables|/Script/Engine.Character|GetCharacterMovement _astoaster))
  (Input|DisableInput _astoaster_controller 0)
  (Utilities|FlowControl|Delay 1.0)
  (UserInterface|CreateWidget "/Game/HUD/LoadingScreen.LoadingScreen_C")
  (Game|SetGamePaused true)
  (Game|OpenLevel(byName) "Outro"))

(fn ConstructionScript)