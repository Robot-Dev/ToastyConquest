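; BP_Fridge is a hackable fridge with a puddle, whose collision box is a hazard to the player's Toaster until hacked.
; Hitting the box damages the Toaster and launches it along the hit normal.
; OnHacked halts the Toaster and disables input during a one-second hacked flipbook and sound.
; It then restores input, destroys the box and swaps flipbooks to show a frozen puddle and after-hack fridge.
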(event OnComponentHit(Box)
  (params (HitComponent :type Primitive%20Component%20Object%20Reference) (OtherActor :type Actor%20Object%20Reference) (OtherComp :type Primitive%20Component%20Object%20Reference) (NormalImpulse :type Vector :default "0, 0, 0") (Hit :type Hit%20Result%20Structure%20%28by%20ref%29))
  (bind _astoaster (Utilities|Casting|CastToToaster OtherActor))
  (Class|Toaster|TakeDamage _astoaster 1.0)
  (Character|LaunchCharacter _astoaster (* (.normal Hit) -1e+03) true true))

(event EventOnHacked
  (bind _returnvalue (Game|GetPlayerController 0))
  (bind _sprite (Variables|Default|GetSprite))
  (bind _astoaster (Utilities|Casting|CastToToaster (Pawn|GetControlledPawn _returnvalue)))
  (bind _astoaster_controller (Utilities|Casting|CastToToasterController _returnvalue))
  (Components|Movement|StopMovementImmediately (Variables|/Script/Engine.Character|GetCharacterMovement _astoaster))
  (Input|DisableInput _astoaster_controller 0)
  (Sprite|SetFlipbook _sprite "/Game/Sprites/Rooms/Kitchen/Sprites/Fridge_Hacked.Fridge_Hacked")
  (Sprite|SetFlipbook (Variables|Default|GetHackable) "/Game/Sprites/Enemies/Granny/Death/Empty.Empty")
  (Audio|PlaySoundatLocation "/Game/Sounds/Other/asset_fridge_v1_Cue.asset_fridge_v1_Cue" (Transformation|GetWorldLocation _sprite))
  (Utilities|FlowControl|Delay 1.0)
  (Input|EnableInput _astoaster_controller 0)
  (Components|DestroyComponent (Variables|Default|GetBox))
  (Sprite|SetFlipbook (Variables|Default|GetPuddle) "/Game/Sprites/Effects/Puddle2/Sprites/louze_frozen.louze_frozen")
  (Sprite|SetFlipbook _sprite "/Game/Sprites/Rooms/Kitchen/Sprites/Fridget_AfterHacked.Fridget_AfterHacked"))

(fn ConstructionScript)