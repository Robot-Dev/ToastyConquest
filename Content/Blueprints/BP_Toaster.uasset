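; BP_Toaster is a side-view actor, apparently the player's toaster character, that drives HUD, hurt and death feedback.
; On BeginPlay it creates the Toaster widget with a reference to itself.
; OnHurt plays a world camera shake at the side-view camera.
; OnDeath removes that widget, pauses the game, shows the Toasted screen with death music, then swaps it for DeathMenu after a delay.
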(event EventBeginPlay
  (bind _returnvalue (UserInterface|CreateWidget "/Game/HUD/Toaster.Toaster_C"))
  (Variables|/Game/HUD/Toaster.Toaster_C|SetToaster _returnvalue self)
  (UserInterface|Viewport|AddtoViewport _returnvalue 0))

(event EventOnHurt
  (Camera|PlayWorldCameraShake "/Game/Blueprints/BP_HurtShake.BP_HurtShake_C" (Transformation|GetWorldLocation (Variables|Default|GetSideViewCameraComponent)) 0.0 1e+03 0.01))

(event EventOnDeath
  (Widget|RemovefromParent (stale EventBeginPlay _returnvalue))
  (Game|SetGamePaused true)
  (bind _returnvalue (UserInterface|CreateWidget "/Game/HUD/Toasted.Toasted_C"))
  (UserInterface|Viewport|AddtoViewport _returnvalue 0)
  (Audio|PlaySound2D "/Game/Sounds/Music/Base/music_death_v1.music_death_v1")
  (Utilities|FlowControl|Delay 4.0)
  (Widget|RemovefromParent _returnvalue)
  (bind _returnvalue_2 (UserInterface|CreateWidget "/Game/HUD/DeathMenu.DeathMenu_C"))
  (UserInterface|Viewport|AddtoViewport _returnvalue_2 0))

(fn ConstructionScript)