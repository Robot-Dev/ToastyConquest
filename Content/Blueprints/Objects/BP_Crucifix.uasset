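; BP_Crucifix is a Paper2D flipbook object that turns into a BP_Life actor when hit by a Toast projectile.
; Overlapping its collision component makes the Toast explode, stops its movement and removes its gravity, then switches the crucifix sprite to the Krucifix flipbook.
; After a short delay, it spawns BP_Life at its own location and destroys itself.
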(event OnComponentBeginOverlap(CollisionComponent)
  (params (OverlappedComponent :type Primitive%20Component%20Object%20Reference) (OtherActor :type Actor%20Object%20Reference) (OtherComp :type Primitive%20Component%20Object%20Reference) (OtherBodyIndex :type Integer) (bFromSweep :type Boolean) (SweepResult :type Hit%20Result%20Structure%20%28by%20ref%29))
  (bind _astoast (Utilities|Casting|CastToToast OtherActor))
  (Class|Toast|Explode _astoast)
  (Components|Movement|StopMovementImmediately (Variables|/Script/ToastyConquest.Projectile|GetProjectileMovement _astoast))
  (Variables|/Script/Engine.ProjectileMovementComponent|SetProjectileGravityScale (Variables|/Script/ToastyConquest.Projectile|GetProjectileMovement _astoast) 0.0)
  (Sprite|SetFlipbook (Variables|Default|GetSprite) "/Game/Sprites/Rooms/LivingRoom/Sprites/Krucifix.Krucifix")
  (Utilities|FlowControl|Delay 0.5)
  (Game|SpawnActorfromClass "/Game/Blueprints/BP_Life.BP_Life_C" (Math|Transform|MakeTransform (.Location (Math|Transform|BreakTransform (Transformation|GetActorTransform)))) "AdjustIfPossibleButAlwaysSpawn" 0 0)
  (Actor|DestroyActor))

(fn ConstructionScript)