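; BP_Soap is a slippery soap object that sends the Toaster character sliding when touched.
; An overlap on its collision component launches the Toaster along its capsule's forward vector, overriding horizontal velocity while adding to vertical.
; It then switches the flipbook sprite to a slip animation, plays a soap sound and returns to idle after a short delay.
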(event OnComponentBeginOverlap(CollisionComponent)
  (params (OverlappedComponent :type Primitive%20Component%20Object%20Reference) (OtherActor :type Actor%20Object%20Reference) (OtherComp :type Primitive%20Component%20Object%20Reference) (OtherBodyIndex :type Integer) (bFromSweep :type Boolean) (SweepResult :type Hit%20Result%20Structure%20%28by%20ref%29))
  (bind _sprite (Variables|Default|GetSprite))
  (bind _astoaster (Utilities|Casting|CastToToaster OtherActor))
  (Character|LaunchCharacter _astoaster (* (Math|Vector|GetForwardVector (Variables|/Script/Engine.Character|GetCapsuleComponent _astoaster)) 3e+03) true false)
  (Sprite|SetFlipbook _sprite "/Game/Sprites/Rooms/Bathroom/Sprites/Soap_Slip.Soap_Slip")
  (Audio|PlaySoundatLocation "/Game/Sounds/Other/asset_soap_v1_Cue.asset_soap_v1_Cue" (Transformation|GetWorldLocation _sprite))
  (Utilities|FlowControl|Delay 0.4)
  (Sprite|SetFlipbook _sprite "/Game/Sprites/Rooms/Bathroom/Sprites/Soap_Idle.Soap_Idle"))

(fn ConstructionScript)