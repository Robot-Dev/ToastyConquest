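; BP_Stairs is a hackable door that reveals stairs leading to Level1.
; OnHacked stops the player Toaster and disables input for one second, then swaps the switch, hackable and main sprite flipbooks, plays a lever sound and destroys the door collision.
; When a Toaster overlaps the collision component, it shows a LoadingScreen widget and opens Level1 after a short delay.
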(event OnComponentBeginOverlap(CollisionComponent)
  (params (OverlappedComponent :type Primitive%20Component%20Object%20Reference) (OtherActor :type Actor%20Object%20Reference) (OtherComp :type Primitive%20Component%20Object%20Reference) (OtherBodyIndex :type Integer) (bFromSweep :type Boolean) (SweepResult :type Hit%20Result%20Structure%20%28by%20ref%29))
  (Utilities|Casting|CastToToaster OtherActor)
  (bind _returnvalue (UserInterface|CreateWidget "/Game/HUD/LoadingScreen.LoadingScreen_C"))
  (UserInterface|Viewport|AddtoViewport _returnvalue 0)
  (Utilities|FlowControl|Delay 0.5)
  (Game|OpenLevel(byName) "Level1"))

(event EventOnHacked
  (bind _returnvalue (Game|GetPlayerController 0))
  (bind _astoaster (Utilities|Casting|CastToToaster (Pawn|GetControlledPawn _returnvalue)))
  (bind _astoaster_controller (Utilities|Casting|CastToToasterController _returnvalue))
  (Components|Movement|StopMovementImmediately (Variables|/Script/Engine.Character|GetCharacterMovement _astoaster))
  (Input|DisableInput _astoaster_controller 0)
  (Utilities|FlowControl|Delay 1.0)
  (Input|EnableInput _astoaster_controller 0)
  (Sprite|SetFlipbook (Variables|Default|GetSwitch) "/Game/Sprites/Rooms/Cellar/Sprites/switch_hacked.switch_hacked")
  (Sprite|SetFlipbook (Variables|Default|GetHackable) "/Game/Sprites/Enemies/Granny/Death/Empty.Empty")
  (Sprite|SetFlipbook (Variables|Default|GetSprite) "/Game/Sprites/Rooms/Cellar/Background/Sprites/Stairs.Stairs")
  (Audio|PlaySoundatLocation "/Game/Sounds/Other/asset_lever_v1_Cue.asset_lever_v1_Cue" (Transformation|GetWorldLocation (Variables|Default|GetSprite)))
  (Components|DestroyComponent (Variables|Default|GetDoorCollision)))

(fn ConstructionScript)