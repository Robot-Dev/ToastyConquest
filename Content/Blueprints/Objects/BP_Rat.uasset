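; BP_Rat is a sprite-based rat hazard that hurts the Toaster character on contact.
; A collision hit deals damage to the Toaster and launches it along the inverted hit normal, overriding its velocity.
; Tick flips the sprite by rotation according to the sign of the rat's X velocity.
; EndPlay stops the bite sound and plays a death sound at the sprite's location.
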(event OnComponentHit(CollisionComponent)
  (params (HitComponent :type Primitive%20Component%20Object%20Reference) (OtherActor :type Actor%20Object%20Reference) (OtherComp :type Primitive%20Component%20Object%20Reference) (NormalImpulse :type Vector :default "0, 0, 0") (Hit :type Hit%20Result%20Structure%20%28by%20ref%29))
  (bind _astoaster (Utilities|Casting|CastToToaster OtherActor))
  (Class|Toaster|TakeDamage _astoaster 1.0)
  (Character|LaunchCharacter _astoaster (* (.normal Hit) -1e+03) true true))

(event EventEndPlay
  (params (EndPlayReason :type EEndPlayReason%20Enum :default "Destroyed"))
  (Audio|Components|Audio|Stop (Variables|Default|GetBiteSound))
  (Audio|PlaySoundatLocation "/Game/Sounds/Other/rat_death_v1_Cue.rat_death_v1_Cue" (Transformation|GetWorldLocation (Variables|Default|GetSprite))))

(event EventTick
  (params (DeltaSeconds :type Float%20%28single-precision%29))
  (bind _sprite (Variables|Default|GetSprite))
  (if (> (.X (Math|Vector|BreakVector (Transformation|GetVelocity))) 0.0)
    (Transformation|SetRelativeRotation _sprite "0, 0, 0" false false)
    (else
      (Transformation|SetRelativeRotation _sprite "0,180.000000, 0" false false))))

(fn ConstructionScript)