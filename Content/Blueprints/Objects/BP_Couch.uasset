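; BP_Couch is a bounce-pad couch that launches the Toaster character straight up when it hits the couch's Box.
; The hit overrides the Toaster's velocity with a fixed upward launch and switches the sprite to its launch flipbook.
; If the sound is not already playing, it plays it and restores the idle flipbook after a short delay.
; BeginPlay stops the audio so it starts silent.
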(event OnComponentHit(Box)
  (params (HitComponent :type Primitive%20Component%20Object%20Reference) (OtherActor :type Actor%20Object%20Reference) (OtherComp :type Primitive%20Component%20Object%20Reference) (NormalImpulse :type Vector :default "0, 0, 0") (Hit :type Hit%20Result%20Structure%20%28by%20ref%29))
  (bind _sprite (Variables|Default|GetSprite))
  (bind _audio (Variables|Default|GetAudio))
  (bind _astoaster (Utilities|Casting|CastToToaster OtherActor))
  (Character|LaunchCharacter _astoaster "0, 0,1600.000000" true true)
  (Sprite|SetFlipbook _sprite "/Game/Sprites/Rooms/Kitchen/Sprites/Divan_Launch.Divan_Launch")
  (if (not (Audio|Components|Audio|IsPlaying _audio))
    (Audio|Components|Audio|Play _audio 0.0)
    (Utilities|FlowControl|Delay 0.5)
    (Sprite|SetFlipbook _sprite "/Game/Sprites/Rooms/Kitchen/Sprites/Divan_Idle.Divan_Idle")))

(event EventBeginPlay
  (Audio|Components|Audio|Stop (Variables|Default|GetAudio)))

(fn ConstructionScript)