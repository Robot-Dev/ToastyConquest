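; BP_Stove is a stove hazard that hurts the Toaster character and knocks it away on contact.
; On BeginPlay it offsets the playback position of its four flame components so their animations are staggered.
; A hit on the Box component by a Toaster deals damage and launches it along the reversed hit normal, overriding its current velocity.
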(event OnComponentHit(Box)
  (params (HitComponent :type Primitive%20Component%20Object%20Reference) (OtherActor :type Actor%20Object%20Reference) (OtherComp :type Primitive%20Component%20Object%20Reference) (NormalImpulse :type Vector :default "0, 0, 0") (Hit :type Hit%20Result%20Structure%20%28by%20ref%29))
  (bind _astoaster (Utilities|Casting|CastToToaster OtherActor))
  (Class|Toaster|TakeDamage _astoaster 1.0)
  (Character|LaunchCharacter _astoaster (* (.normal Hit) -1e+03) true true))

(event EventBeginPlay
  (Components|Timeline|SetPlaybackPosition (Variables|Default|GetFlame) 0.0 false)
  (Components|Timeline|SetPlaybackPosition (Variables|Default|GetFlame2) 1.0 false)
  (Components|Timeline|SetPlaybackPosition (Variables|Default|GetFlame3) 2.0 false)
  (Components|Timeline|SetPlaybackPosition (Variables|Default|GetFlame4) 3.0 false))

(fn ConstructionScript)