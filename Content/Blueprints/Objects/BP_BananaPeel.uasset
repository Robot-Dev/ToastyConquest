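; BP_BananaPeel is a banana peel hazard that sends the Toaster character sliding when stepped on.
; On collision overlap with a Toaster, it launches the character along its capsule's forward vector, adding to current velocity rather than overriding it.
; It also swaps its sprite to a slip flipbook and plays a sound at its location, then restores the idle flipbook after a short delay.
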(event OnComponentBeginOverlap(CollisionComponent)
  (params (OverlappedComponent :type Primitive%20Component%20Object%20Reference) (OtherActor :type Actor%20Object%20Reference) (OtherComp :type Primitive%20Component%20Object%20Reference) (OtherBodyIndex :type Integer) (bFromSweep :type Boolean) (SweepResult :type Hit%20Result%20Structure%20%28by%20ref%29))
  (bind _sprite (Variables|Default|GetSprite))
  (bind _astoaster (Utilities|Casting|CastToToaster OtherActor))
  (Character|LaunchCharacter _astoaster (* (Math|Vector|GetForwardVector (Variables|/Script/Engine.Character|GetCapsuleComponent _astoaster)) 3e+03) false false)
  (Sprite|SetFlipbook _sprite "/Game/Sprites/Rooms/Kitchen/Sprites/Banana_Slip.Banana_Slip")
  (Audio|PlaySoundatLocation "/Game/Sounds/Other/asset_banana_v1_Cue_2.asset_banana_v1_Cue_2" (Transformation|GetWorldLocation (Variables|Default|GetSprite)))
  (Utilities|FlowControl|Delay 0.4)
  (Sprite|SetFlipbook _sprite "/Game/Sprites/Rooms/Kitchen/Sprites/Banana_Idle.Banana_Idle"))

(event EventBeginPlay)

(event Collision|EventActorBeginOverlap
  (params (OtherActor :type Actor%20Object%20Reference)))

(fn ConstructionScript)